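; Enemy spider pawn that endlessly chases the player and attacks in melee range.
; BeginPlay loops AI MoveTo with a short retry delay, while Tick plays the attack montage, disabling movement during it to prevent sliding.
; Damage reduces health until death stops movement and collision, credits BP_Marine with a kill, then destroys the actor after a delay.
; DamagePlayer applies hit damage but is not called within this Blueprint.
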(event `self.ReceiveBeginPlay`
  ;[1 1 1] AI movement set to chase player indefinitely
  (if (`self.Is Alive`) :!label _label
    (`|AIMoveTo` self (0.0 0.0 0.0) (`GameplayStatics.GetPlayerCharacter` 0)
      (:`OnSuccess`
        _)
      (:`OnFail`
        _))
    (`KismetSystemLibrary.Delay` 0.2)
    (goto _label)))

(event `self.ReceiveAnyDamage`
  (params (Damage :type "Float (single-precision)") (DamageType :type "DamageType Object Reference") (InstigatedBy :type "Controller Object Reference") (DamageCauser :type "Actor Object Reference"))
  ;[1 1 1] Damage and death
  (if (`self.Is Alive`)
    (`self.Decrease Health` Damage)
    (if (== (`self.Health`) 0.0)
      (`self.Kill AI`)
      (`KismetSystemLibrary.Delay` 3.0)
      (`self.K2_DestroyActor`))))

(event `self.ReceiveTick`
  (params (DeltaSeconds :type "Float (single-precision)"))
  ;[1 1 1] Check if player is within attack range as well as if spider is already attacking
  (if (and (`self.Is Within Attack Range`) (not (`self.Is Attacking`)) (`self.Is Alive`))
    ;[1 1 1] Prevents spider from sliding towards player while attacking
    (`ActorComponent.Deactivate` (`self.CharacterMovement`))
    (`|PlayMontage` (`self.Mesh`) "/Game/Characters/Enemy_Great_Spider/Animations/SpiderAttack1.SpiderAttack1"
      (:`OnCompleted`
        (`ActorComponent.Activate` (`self.CharacterMovement`) false)))))

(fn `Damage Player`
  (`GameplayStatics.ApplyDamage` (`GameplayStatics.GetPlayerCharacter` 0) (`self.Damage Per Hit`)))

(fn `Decrease Health`
  (params (`Damage Amount` :type "Float (double-precision)"))
  (set `self.Health` (`KismetMathLibrary.FClamp` (- (`self.Health`) `Damage Amount`) 0.0 100.0)))

(fn `Is Alive`
  (returns (ReturnValue :type Boolean))
  (return (not (`self.isDead`))))

(fn `Is Attacking`
  (returns (ReturnValue :type Boolean))
  (return (`AnimInstance.Montage_IsPlaying` (`SkeletalMeshComponent.GetAnimInstance` (`self.Mesh`)) "/Game/Characters/Enemy_Great_Spider/Animations/SpiderAttack1.SpiderAttack1")))

(fn `Is Within Attack Range`
  (returns (ReturnValue :type Boolean))
  (return (< (`self.GetDistanceTo` (`GameplayStatics.GetPlayerCharacter` 0)) (`self.AttackRange`))))

(fn `Kill AI`
  (bind _charactermovement (`self.CharacterMovement`))
  (set `self.isDead` true)
  (`MovementComponent.StopMovementImmediately` _charactermovement)
  (`ActorComponent.Deactivate` _charactermovement)
  (`self.SetActorEnableCollision` false)
  (bind _asbp_marine (cast `/Game/Blueprints/Pawns/BP_Marine` (`GameplayStatics.GetPlayerCharacter` 0)))
  (`/Game/Blueprints/Pawns/BP_Marine.Increase Kills` _asbp_marine))

(fn `UserConstructionScript`)